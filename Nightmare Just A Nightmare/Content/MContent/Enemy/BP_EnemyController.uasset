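; Enemy AI controller that starts BT_Enemy on BeginPlay and feeds it what AI Perception detects.
; Each perception update runs through touch, sight, hearing and prediction handlers, which filter by sense class and write to the Blackboard.
; Sight and touch set or clear the player as TargetActor, while hearing sets TargetLocation.
; Losing sight of the player requests a pawn prediction, whose stimulus location becomes LastKnownLocation.
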(event OnTargetPerceptionUpdated(AIPerception)
  (params (Actor :type Actor%20Object%20Reference) (Stimulus :type AI%20Stimulus%20Structure))
  ;[1 1 1] Triggers every time if is in sight & if lose sight
  (CallFunction|TouchSense Actor Stimulus)
  (CallFunction|SightSense Actor Stimulus)
  (CallFunction|HearSense Stimulus)
  (CallFunction|Prediction Stimulus))

(event EventBeginPlay
  (AI|RunBehaviorTree "/Game/MContent/Enemy/BT_Enemy.BT_Enemy"))

(fn ConstructionScript)

(fn SightSense
  (params (Actor :type Actor%20Object%20Reference) (Stimulus :type AI%20Stimulus%20Structure))
  ;[1 1 1] Fire Twice (When in sight and when not in sight)
  (bind _returnvalue (Class|AIPerceptionSystem|GetSenseClassforStimulus Stimulus))
  (if (== _returnvalue "/Script/AIModule.AISense_Sight")
    (if (== Actor (Game|GetPlayerCharacter 0))
      ;[1 1 1] Set Player object as A value
      (AI|Components|Blackboard|SetValueasObject (Variables|Default|GetBlackboard) (Utilities|Name|MakeLiteralName "TargetActor") (Utilities|SelectObject (Game|GetPlayerCharacter 0) 0 (.bsuccessfullysensed Stimulus)))
      (if (not (.bsuccessfullysensed Stimulus))
        (Class|AISensePrediction|RequestPawnPredictionEvent (Pawn|GetControlledPawn) (Game|GetPlayerCharacter 0) 1.0))
      (else
        (return)))
    (else
      (return))))

(fn HearSense
  (params (Stimulus :type AI%20Stimulus%20Structure%20%28by%20ref%29))
  (bind _returnvalue (Class|AIPerceptionSystem|GetSenseClassforStimulus Stimulus))
  (if (== _returnvalue "/Script/AIModule.AISense_Hearing")
    (AI|Components|Blackboard|SetValueasVector (Variables|Default|GetBlackboard) (Utilities|Name|MakeLiteralName "TargetLocation") (.StimulusLocation (Utilities|Struct|BreakAIStimulus Stimulus)))))

(fn TouchSense
  (params (Actor :type Actor%20Object%20Reference) (Stimulus :type AI%20Stimulus%20Structure))
  (bind _returnvalue (Class|AIPerceptionSystem|GetSenseClassforStimulus Stimulus))
  (if (== _returnvalue "/Script/AIModule.AISense_Touch")
    (if (== Actor (Game|GetPlayerCharacter 0))
      ;[1 1 1] Set Player object as A value
      (AI|Components|Blackboard|SetValueasObject (Variables|Default|GetBlackboard) (Utilities|Name|MakeLiteralName "TargetActor") (Utilities|SelectObject (Game|GetPlayerCharacter 0) 0 (.bsuccessfullysensed Stimulus)))
      (else
        (return)))
    (else
      (return))))

(fn Prediction
  (params (Stimulus :type AI%20Stimulus%20Structure%20%28by%20ref%29))
  (bind _returnvalue (Class|AIPerceptionSystem|GetSenseClassforStimulus Stimulus))
  (if (== _returnvalue "/Script/AIModule.AISense_Prediction")
    (AI|Components|Blackboard|SetValueasVector (Variables|Default|GetBlackboard) (Utilities|Name|MakeLiteralName "LastKnownLocation") (.StimulusLocation (Utilities|Struct|BreakAIStimulus Stimulus)))))